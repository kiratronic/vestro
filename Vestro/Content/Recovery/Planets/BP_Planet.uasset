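; BP_Planet is a planet actor with a sphere mesh, a planet radius and a gravity field radius.
; UpdatePlanet scales PlanetSphere and derives GravityFieldRadius from PlanetRadius.
; Disconnected construction-script logic would call it and, for the closest planet, hide the sphere, move and scale VoxelWorld in its place, and recenter the actor at atmosphere scale.
; The construction script and events are empty, so none of this runs from this graph.
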(fn `UpdatePlanet`
  (`SceneComponent.SetWorldScale3D` (`self.PlanetSphere`) (`KismetMathLibrary.Conv_DoubleToVector` (* (`self.Planet Radius`) 2.0 1000.0)))
  (set `self.GravityFieldRadius` (* (`self.Planet Radius`) 1.1 100000.0)))

(fn `UserConstructionScript`)